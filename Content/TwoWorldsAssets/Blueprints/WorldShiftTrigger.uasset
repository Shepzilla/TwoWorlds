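; WorldShiftTrigger is a trigger Blueprint meant to shift between physical and spirit worlds, but currently it only starts the physical-world music on BeginPlay.
; Its overlap event is empty, leaving disconnected the logic that would toggle InSpirit, call ChangeMusic and swap every StaticMeshActor's first material.
; ChangeMusic restarts music through a FlipFlop, though both branches select the spiritual-world track.
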(event `self.ReceiveBeginPlay`
  (`AudioComponent.SetSound` (`self.BackgroundMusic`) "/Game/TwoWorldsAssets/Sounds/Music_Physical_World.Music_Physical_World")
  (`AudioComponent.Play` (`self.BackgroundMusic`) 0.0))

(event `self.ReceiveActorBeginOverlap`
  (params (OtherActor :type "Actor Object Reference"))
  ;[1 1 1] Detects if player has entered trigger.
)

(event `Change music`
  (`/Engine/EditorBlueprintResources/StandardMacros.FlipFlop`
    (:`A`
      (`AudioComponent.Stop` (`self.BackgroundMusic`))
      (`AudioComponent.SetSound` (`self.BackgroundMusic`) "/Game/TwoWorldsAssets/Sounds/Music_Spiritual_World.Music_Spiritual_World")
      (`AudioComponent.Play` (`self.BackgroundMusic`) 0.0))
    (:`B`
      (`AudioComponent.Stop` (`self.BackgroundMusic`))
      (`AudioComponent.SetSound` (`self.BackgroundMusic`) "/Game/TwoWorldsAssets/Sounds/Music_Spiritual_World.Music_Spiritual_World")
      (`AudioComponent.Play` (`self.BackgroundMusic`) 0.0))))

(fn `UserConstructionScript`)