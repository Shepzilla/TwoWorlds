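; Background music actor that plays the track for the world the player is in, physical or spiritual.
; On BeginPlay it starts the physical world music on its audio component.
; Its Changemusic event reads InSpirit from the first GlobalController in the level, then stops the audio and restarts it with the matching world's track from the beginning.
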(event `self.ReceiveBeginPlay`
  (`AudioComponent.SetSound` (`self.BackgroundMusic`) "/Game/TwoWorldsAssets/Sounds/Music_Physical_World.Music_Physical_World")
  (`AudioComponent.Play` (`self.BackgroundMusic`) 0.0))

(event `Change music`
  (bind _outactors (`GameplayStatics.GetAllActorsOfClass` "/Game/TwoWorldsAssets/Blueprints/GlobalController.GlobalController_C"))
  (if (`/Game/TwoWorldsAssets/Blueprints/GlobalController.InSpirit?` (`KismetArrayLibrary.Array_Get` _outactors))
    (`AudioComponent.Stop` (`self.BackgroundMusic`))
    (`AudioComponent.SetSound` (`self.BackgroundMusic`) "/Game/TwoWorldsAssets/Sounds/Music_Spiritual_World.Music_Spiritual_World")
    (`AudioComponent.Play` (`self.BackgroundMusic`) 0.0)
    (else
      (`AudioComponent.Stop` (`self.BackgroundMusic`))
      (`AudioComponent.SetSound` (`self.BackgroundMusic`) "/Game/TwoWorldsAssets/Sounds/Music_Physical_World.Music_Physical_World")
      (`AudioComponent.Play` (`self.BackgroundMusic`) 0.0))))

(fn `UserConstructionScript`)